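; BP_LoadedLevelGameMode is a game mode that, on BeginPlay, trims the level's playable characters to match the one selected in the Venari game instance.
; It finds the Agile and Berserker character actors and destroys the first instance of each type that does not match CurrentCharacter, with no check for an empty result.
; It then hides the notebook; Tick and the construction script add no logic.
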(event EventBeginPlay
  (|CallParentFunction)
  (Utilities|FlowControl|Sequence
    (:then_0
      (bind _outactors (Actor|GetAllActorsOfClass "/Game/01_Blueprints/BP_AgileCharacter.BP_AgileCharacter_C"))
      (if (not (Utilities|Enum|Equal(Enum) (Variables|/Script/ProjectM.VenariGameInstance|GetCurrentCharacter (CallFunction|GetVenariGameInstance)) "AGILE"))
        (Actor|DestroyActor (Utilities|Array|Get(acopy) _outactors))))
    (:then_1
      (bind _outactors_2 (Actor|GetAllActorsOfClass "/Game/01_Blueprints/BP_BerserkerCharacter.BP_BerserkerCharacter_C"))
      (if (not (Utilities|Enum|Equal(Enum) (Variables|/Script/ProjectM.VenariGameInstance|GetCurrentCharacter (CallFunction|GetVenariGameInstance)) "BERSERKER"))
        (Actor|DestroyActor (Utilities|Array|Get(acopy) _outactors_2))))
    (:then_2
      (CallFunction|SetNotebookVisibility false))))

(event EventTick
  (params (DeltaSeconds :type Float%20%28single-precision%29))
  (|CallParentFunction DeltaSeconds) ; This node is disabled and will not be called.\nDrag off pins to build functionality.
)

(fn ConstructionScript
  (|CallParentFunction))