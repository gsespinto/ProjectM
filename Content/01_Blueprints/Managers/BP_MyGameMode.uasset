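; Game mode that sets up the player's UI and chosen character when play begins.
; BeginPlay adds the main HUD, kept in PlayerUI, and the notebook widget to the viewport, then unpossesses the first player controller's pawn.
; It reads CurrentCharacter from the Venari game instance and possesses the first Agile or Berserker character found in the level to match, rather than spawning one.
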(event EventBeginPlay
  (bind _returnvalue (UserInterface|CreateWidget "/Game/01_Blueprints/WBP_MainHUD.WBP_MainHUD_C"))
  (bind _output_get (Variables|Default|SetPlayerUI _returnvalue))
  (UserInterface|Viewport|AddtoViewport _output_get 0)
  (bind _returnvalue_2 (UserInterface|CreateWidget "/Game/01_Blueprints/Notebook/WBP_Notebook.WBP_Notebook_C"))
  (UserInterface|Viewport|AddtoViewport _returnvalue_2 0)
  (Pawn|UnPossess (Game|GetPlayerController 0))
  (Utilities|FlowControl|Sequence
    (:then_0
      (bind _outactors (Actor|GetAllActorsOfClass "/Game/01_Blueprints/BP_AgileCharacter.BP_AgileCharacter_C"))
      (if (Utilities|Enum|Equal(Enum) (Variables|/Script/ProjectM.VenariGameInstance|GetCurrentCharacter (CallFunction|GetVenariGameInstance)) "AGILE")
        (Pawn|Possess (Game|GetPlayerController 0) (Utilities|Array|Get(acopy) _outactors))))
    (:then_1
      (bind _outactors_2 (Actor|GetAllActorsOfClass "/Game/01_Blueprints/BP_BerserkerCharacter.BP_BerserkerCharacter_C"))
      (if (Utilities|Enum|Equal(Enum) (Variables|/Script/ProjectM.VenariGameInstance|GetCurrentCharacter (CallFunction|GetVenariGameInstance)) "BERSERKER")
        (Pawn|Possess (Game|GetPlayerController 0) (Utilities|Array|Get(acopy) _outactors_2))))))

(event EventTick
  (params (DeltaSeconds :type Float%20%28single-precision%29)))

(fn ConstructionScript)