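; BP_Barrel is an exploding barrel that damages an enemy when its mesh hits one.
; On BeginPlay it binds to the static mesh's hit event and reacts only to actors tagged "Enemy".
; A sequence tries both ProjectMCharacter and Enemy casts; a successful cast applies DamageAmount to that actor alone, plays explosion FX and destroys the barrel.
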(event Custom|OnComponentHit_Event_0
  (params (HitComponent :type Primitive%20Component%20Object%20Reference) (OtherActor :type Actor%20Object%20Reference) (OtherComp :type Primitive%20Component%20Object%20Reference) (NormalImpulse :type Vector) (Hit :type Hit%20Result%20Structure%20%28by%20ref%29))
  (Utilities|IsValid OtherActor
    (:Is%20Valid
      (if (Actor|ActorHasTag OtherActor "Enemy")
        (Utilities|FlowControl|Sequence
          (:then_0
            (bind _asproject_mcharacter (Utilities|Casting|CastToProjectMCharacter OtherActor))
            (Class|ProjectMCharacter|TakeDamage _asproject_mcharacter (Variables|Default|GetDamageAmount)))
          (:then_1
            (bind _asenemy (Utilities|Casting|CastToEnemy OtherActor))
            (Class|Enemy|TakeDamage _asenemy (Variables|Default|GetDamageAmount))))
        (CallFunction|PlayExplosionFX (Transformation|GetActorLocation))
        (Actor|DestroyActor)))))

(event EventBeginPlay
  (Collision|AssignOnComponentHit (Variables|Default|GetStaticMesh) (delegate Custom|OnComponentHit_Event_0)))

(event Collision|EventActorBeginOverlap
  (params (OtherActor :type Actor%20Object%20Reference)))

(event EventTick
  (params (DeltaSeconds :type Float%20%28single-precision%29)))

(fn ConstructionScript)