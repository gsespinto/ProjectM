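; Grapple hook point actor that shows an AgileCharacter player a detection widget and supplies a landing point.
; While active, Tick scales the fill with player distance, switching from grey to a type color (grapple, pull, enemy) within throw range.
; Use plays an animation and pauses fill updates until a timer resets it.
; Player overlap with the Box disables Sphere collision and marks the point unusable.
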(event OnComponentBeginOverlap(Box)
  (params (OverlappedComponent :type Primitive%20Component%20Object%20Reference) (OtherActor :type Actor%20Object%20Reference) (OtherComp :type Primitive%20Component%20Object%20Reference) (OtherBodyIndex :type Integer) (bFromSweep :type Boolean) (SweepResult :type Hit%20Result%20Structure%20%28by%20ref%29))
  (if (== OtherActor (Variables|Default|GetPawnRef))
    (Collision|SetCollisionEnabled (Variables|Default|GetSphere) "NoCollision")
    (Variables|Default|SetbCanBeUsed false)))

(event OnComponentEndOverlap(Box)
  (params (OverlappedComponent :type Primitive%20Component%20Object%20Reference) (OtherActor :type Actor%20Object%20Reference) (OtherComp :type Primitive%20Component%20Object%20Reference) (OtherBodyIndex :type Integer))
  (if (== OtherActor (Variables|Default|GetPawnRef))
    (Collision|SetCollisionEnabled (Variables|Default|GetSphere) "QueryAndPhysics")
    (Variables|Default|SetbCanBeUsed true)))

(event EventBeginPlay
  (bind _aswbp_detection_node (Utilities|Casting|CastToWBP_DetectionNode (UserInterface|GetUserWidgetObject (Variables|Default|GetWidget))))
  (Variables|Default|SetWidgetRef _aswbp_detection_node)
  (bind _asagile_character (Utilities|Casting|CastToAgileCharacter (Game|Player|GetPlayerPawn 0))
    (:then
      (Variables|Default|SetPawnRef _asagile_character))
    (:CastFailed
      _))
  (CallFunction|Deactivate)
  (CallFunction|SetInitialSizeBrushes)
  (CallFunction|SetTypeColor))

(event Collision|EventActorBeginOverlap
  (params (OtherActor :type Actor%20Object%20Reference)))

(event EventTick
  (params (DeltaSeconds :type Float%20%28single-precision%29))
  (CallFunction|CheckPlayer)
  (if (and (Variables|Default|GetbActive) (not (Variables|Default|GetbUse)))
    (CallFunction|CheckDistancefromPlayer)))

(fn ConstructionScript)

(fn SetInitialSizeBrushes
  (bind _widgetref (Variables|Default|GetWidgetRef))
  (Class|Image|SetBrushSize (Variables|/Game/01_Blueprints/GrapplingHook/WBP_DetectionNode.WBP_DetectionNode_C|GetBackGround _widgetref) (Math|Vector2D|MakeVector2D 5e+01 5e+01))
  (Class|Image|SetBrushSize (Variables|/Game/01_Blueprints/GrapplingHook/WBP_DetectionNode.WBP_DetectionNode_C|GetFill _widgetref)))

(fn Use
  (bind _widgetref (Variables|Default|GetWidgetRef))
  (Variables|Default|SetbUse true)
  (UserInterface|Animation|PlayAnimation _widgetref (Variables|/Game/01_Blueprints/GrapplingHook/WBP_DetectionNode.WBP_DetectionNode_C|GetNodeUse _widgetref) 0.0 1 "Forward" 1.0 true)
  (Utilities|Time|SetTimerbyFunctionName 0 "Reactivate" 2.0))

(fn Deactivate
  (Variables|Default|SetbActive false)
  (Widget|SetVisibility (Variables|Default|GetWidgetRef) "Hidden"))

(fn CheckDistancefromPlayer
  (bind _returnvalue (Transformation|GetActorLocation))
  (bind _pawnref (Variables|Default|GetPawnRef))
  (bind _pawnref_2 (Variables|Default|GetPawnRef))
  (bind _widgetref (Variables|Default|GetWidgetRef))
  (bind _returnvalue_2 (Transformation|GetActorLocation _pawnref))
  (bind _fill (Variables|/Game/01_Blueprints/GrapplingHook/WBP_DetectionNode.WBP_DetectionNode_C|GetFill _widgetref))
  (bind _grapplethrowdistance (Variables|/Script/ProjectM.AgileCharacter|GetGrappleThrowDistance _pawnref_2))
  (bind _detectiondistance (Variables|/Script/ProjectM.AgileCharacter|GetDetectionDistance _pawnref_2))
  (bind _returnvalue_3 (- _returnvalue_2 _returnvalue))
  (bind _returnvalue_4 (Math|Vector|VectorLength _returnvalue_3))
  (bind _returnvalue_5 (Math|Float|MapRangeClamped _returnvalue_4 _grapplethrowdistance _detectiondistance 4e+01 5.0))
  (Class|Image|SetBrushSize _fill (Math|Vector2D|MakeVector2D _returnvalue_5 _returnvalue_5))
  (Appearance|SetColorandOpacity _fill (Math|Color|SelectColor (Math|Conversions|ToLinearColor(Color) (Variables|Default|GetTargetColor)) "(R=0.630208,G=0.630208,B=0.630208,A=1.000000)" (== _returnvalue_5 4e+01)) :!class /Script/UMG.Image))

(fn Reactivate
  (Variables|Default|SetbUse false))

(fn Activate
  (params (PawnRef :type Agile%20Character%20Object%20Reference))
  (Variables|Default|SetbActive true)
  (Widget|SetVisibility (Variables|Default|GetWidgetRef) "Visible")
  (Variables|Default|SetPawnRef PawnRef))

(fn CanUse
  (return (Variables|Default|GetbCanBeUsed)))

(fn CheckPlayer
  (bind _widget (Variables|Default|GetWidget))
  (Utilities|Casting|CastToAgileCharacter (Game|Player|GetPlayerPawn 0)
    (:then
      (Rendering|SetVisibility _widget true false))
    (:CastFailed
      (Rendering|SetVisibility _widget false false))))

(fn SetTypeColor
  (switch int (Math|Conversions|ToInteger(Byte) (Variables|Default|GetType))
    (:Default
      (Variables|Default|SetTargetColor (Variables|Default|GetGrappleColor) :!label _label))
    (:0
      (goto _label))
    (:1
      (Variables|Default|SetTargetColor (Variables|Default|GetPullColor)))
    (:2
      (Variables|Default|SetTargetColor (Variables|Default|GetEnemyColor)))))

(fn GetLandingPoint
  (|CallParentFunction)
  (return (Variables|Default|GetScene)))