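; BP_BearTrap is a placeable inventory trap that damages characters stepping into it, explodes and destroys itself.
; UseItem removes one "ExplosiveTrap" item via DT_ItemsData, plays a sound, then swaps the preview mesh for the trap mesh at its transform and enables the trigger box.
; Box overlap damages Enemy or ProjectMCharacter actors before the explosion effect.
; PlayerCharacter overlaps do nothing, as that damage branch is disconnected.
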(event OnComponentBeginOverlap(Box)
  (params (OverlappedComponent :type Primitive%20Component%20Object%20Reference) (OtherActor :type Actor%20Object%20Reference) (OtherComp :type Primitive%20Component%20Object%20Reference) (OtherBodyIndex :type Integer) (bFromSweep :type Boolean) (SweepResult :type Hit%20Result%20Structure%20%28by%20ref%29))
  ;[1 1 1] If a player character steps on the trap
  (bind _asplayer_character (Utilities|Casting|CastToPlayerCharacter OtherActor)
    (:CastFailed
      (bind _asenemy (Utilities|Casting|CastToEnemy OtherActor)
        (:then
          (Class|Enemy|TakeDamage _asenemy (Variables|Default|GetDamageAmount)))
        (:CastFailed
          (bind _asproject_mcharacter (Utilities|Casting|CastToProjectMCharacter OtherActor))
          (Class|ProjectMCharacter|TakeDamage _asproject_mcharacter (Variables|Default|GetDamageAmount))))
      ;[1 1 1] Explosion VFX
      (CallFunction|PlayExplosionFX (Transformation|GetActorLocation))
      ;[1 1 1] Destroy trap
      (Actor|DestroyActor))))

(event EventBeginPlay)

(event Collision|EventActorBeginOverlap
  (params (OtherActor :type Actor%20Object%20Reference)))

(event EventTick
  (params (DeltaSeconds :type Float%20%28single-precision%29)))

(event EventUseItem
  (params (Player :type Player%20Character%20Object%20Reference))
  (bind _staticmesh (Variables|Default|GetStaticMesh))
  (bind _previewmesh (Variables|Default|GetPreviewMesh))
  ;[1 1 1] Remove item from inventory
  (bind _returnvalue (Utilities|GetDataTableRow "/Game/02_DataTables/DT_ItemsData.DT_ItemsData" "ExplosiveTrap")
    (:then
      (Class|PlayerCharacter|RemoveItem Player _returnvalue 1)
      (Class|PlayerCharacter|Play2DSound Player "/Game/04_Sound/SFX/PlaceBearTrap.PlaceBearTrap" 1.0 1.0)
      ;[1 1 1] Enable trap's mesh and trigger box
      (Development|SetHiddeninGame (Variables|Default|GetStaticMesh) false false)
      (Collision|SetCollisionEnabled (Variables|Default|GetBox) "QueryOnly")
      ;[1 1 1] Hide preview mesh
      (Development|SetHiddeninGame (Variables|Default|GetPreviewMesh) true false)
      ;[1 1 1] Set trap's transform to the same as the preview
      (Transformation|SetWorldLocation _staticmesh (Transformation|GetWorldLocation _previewmesh) false false)
      (Transformation|SetWorldRotation _staticmesh (Transformation|GetWorldRotation _previewmesh) false false)
      ;[1 1 1] Disable physic simulations
      (Physics|SetSimulatePhysics _staticmesh false)
      (CallFunction|ReorderInventoryData))))

(fn ConstructionScript)