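; BP_BearTrap1 is a single-use trap actor in the inventory system that damages a character stepping into its Box collision.
; On overlap it tries casts to PlayerCharacter, Enemy and ProjectMCharacter in turn, applying DamageAmount through TakeDamage to the first match.
; Each successful hit plays an explosion effect at the trap's location and destroys the trap, while other actors leave it untouched.
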(event OnComponentBeginOverlap(Box)
  (params (OverlappedComponent :type Primitive%20Component%20Object%20Reference) (OtherActor :type Actor%20Object%20Reference) (OtherComp :type Primitive%20Component%20Object%20Reference) (OtherBodyIndex :type Integer) (bFromSweep :type Boolean) (SweepResult :type Hit%20Result%20Structure%20%28by%20ref%29))
  ;[1 1 1] If a player character steps on the trap
  (bind _asplayer_character (Utilities|Casting|CastToPlayerCharacter OtherActor)
    (:then
      ;[1 1 1] Give damage
      (Class|PlayerCharacter|TakeDamage _asplayer_character (Variables|Default|GetDamageAmount)))
    (:CastFailed
      (bind _asenemy (Utilities|Casting|CastToEnemy OtherActor)
        (:then
          (Class|Enemy|TakeDamage _asenemy (Variables|Default|GetDamageAmount)))
        (:CastFailed
          (bind _asproject_mcharacter (Utilities|Casting|CastToProjectMCharacter OtherActor))
          (Class|ProjectMCharacter|TakeDamage _asproject_mcharacter (Variables|Default|GetDamageAmount))))))
  ;[1 1 1] Explosion VFX
  (CallFunction|PlayExplosionFX (Transformation|GetActorLocation))
  ;[1 1 1] Destroy trap
  (Actor|DestroyActor))

(fn ConstructionScript)