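; BP_HealthPotionItem is the health potion inventory item, which heals the player on use.
; UseItem calls Heal on the player's HealthComponent, then removes one potion using its DT_ItemsData row.
; If that row is found, it also plays a gulp sound and drink montage, then calls ReorderInventoryData.
; A full-health check exists but is disconnected, so UseItem applies no such guard.
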(event EventBeginPlay)

(event Collision|EventActorBeginOverlap
  (params (OtherActor :type Actor%20Object%20Reference)))

(event EventTick
  (params (DeltaSeconds :type Float%20%28single-precision%29)))

(event EventUseItem
  (params (Player :type Player%20Character%20Object%20Reference))
  ;[1 1 1] Heal player
  (Class|HealthComponent|Heal (Variables|/Script/ProjectM.PlayerCharacter|GetHealthComponent Player) (Variables|Default|GetHealAmount))
  ;[1 1 1] Remove a health potion from the inventory
  (bind _returnvalue (Utilities|GetDataTableRow "/Game/02_DataTables/DT_ItemsData.DT_ItemsData" "HealthPotion")
    (:then
      (Class|PlayerCharacter|RemoveItem Player _returnvalue 1)
      (Class|PlayerCharacter|Play2DSound Player "/Game/04_Sound/SFX/Gulp.Gulp" 0.75 1.0)
      (Animation|Montage|PlayMontage (Variables|/Script/Engine.Character|GetMesh Player) "/Game/03_Geometry/Characters/AM_Drink.AM_Drink"
        (:then
          (CallFunction|ReorderInventoryData))))))

(fn ConstructionScript)