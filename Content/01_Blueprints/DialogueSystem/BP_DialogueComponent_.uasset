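; BP_DialogueComponent is a component that runs a behavior-tree-driven dialogue when a player interacts.
; On BeginPlay it spawns its own BP_DialogueAIController to execute the dialogue tree.
; Interaction shows WBP_DialogueWidget, switches to UI input, stops player movement, runs the tree and passes the widget through the blackboard.
; The widget's exit event restores game input, removes the widget and stops the tree.
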(event Custom|OnExit_Event_0
  (bind _dialogue_widget (Variables|Default|GetDialogue%20Widget))
  (bind _returnvalue (Widget|GetOwningPlayer _dialogue_widget))
  (Input|SetInputModeGameOnly _returnvalue)
  (Variables|/Script/Engine.PlayerController|SetbShowMouseCursor _returnvalue false)
  (Widget|RemovefromParent (Variables|Default|GetDialogue%20Widget))
  (AI|Logic|StopLogic (Variables|/Script/AIModule.AIController|GetBrainComponent (Variables|Default|GetAIController)) ""))

(event EventBeginPlay
  (bind _returnvalue (Game|SpawnActorfromClass "/Game/01_Blueprints/DialogueSystem/BP_DialogueAIController.BP_DialogueAIController_C" (Math|Transform|MakeTransform "0, 0, 0" "0, 0, 0" "1,1,1") "Undefined" 0 0))
  (Variables|Default|SetAIController _returnvalue))

(event EventOnInteraction
  (params (PlayerCharacter :type Player%20Character%20Object%20Reference))
  (bind _asplayer_controller (Game|GetPlayerController PlayerCharacter))
  (bind _aicontroller (Variables|Default|GetAIController))
  (bind _returnvalue (UserInterface|CreateWidget "/Game/01_Blueprints/DialogueSystem/Widgets/WBP_DialogueWidget.WBP_DialogueWidget_C" _asplayer_controller))
  (bind _output_get (Variables|Default|SetDialogue%20Widget _returnvalue))
  (EventDispatchers|AssignOnExit _output_get (delegate Custom|OnExit_Event_0))
  (UserInterface|Viewport|AddtoViewport _output_get 0)
  (Input|SetInputModeUIOnly _asplayer_controller (Variables|/Game/01_Blueprints/DialogueSystem/Widgets/WBP_DialogueWidget.WBP_DialogueWidget_C|GetSpeakBT _output_get) "LockAlways")
  (Variables|/Script/Engine.PlayerController|SetbShowMouseCursor _asplayer_controller true)
  (Components|Movement|StopMovementImmediately (Variables|/Script/Engine.Character|GetCharacterMovement PlayerCharacter))
  (AI|RunBehaviorTree _aicontroller (Variables|Default|GetDialogueTree))
  (bind _blackboardcomponent (Class|AIController|UseBlackboard _aicontroller "/Game/01_Blueprints/DialogueSystem/BB_DialogueBoard.BB_DialogueBoard"))
  (AI|Components|Blackboard|SetValueasObject _blackboardcomponent (Utilities|Name|MakeLiteralName "DialogueWidget") (Variables|Default|GetDialogue%20Widget)))