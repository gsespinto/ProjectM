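; BP_BossTest is a test boss Blueprint that records the defeat of the "Piglet" monster.
; It polls its HealthComponent every Tick rather than reacting to a death event.
; Once dead, while ChildActor is still valid, it adds the hardcoded name uniquely to the Venari game instance's DefeatedMonsters list and destroys the ChildActor component.
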(event EventBeginPlay)

(event Collision|EventActorBeginOverlap
  (params (OtherActor :type Actor%20Object%20Reference)))

(event EventTick
  (params (DeltaSeconds :type Float%20%28single-precision%29))
  (bind _returnvalue (Class|HealthComponent|IsDead (Variables|Default|GetHealthComponent)))
  (if (and _returnvalue (Utilities|IsValid (Variables|Default|GetChildActor)))
    (Utilities|Array|AddUnique (Variables|/Script/ProjectM.VenariGameInstance|GetDefeatedMonsters (CallFunction|GetVenariGameInstance)) "Piglet")
    (Components|DestroyComponent (Variables|Default|GetChildActor))))

(fn ConstructionScript)