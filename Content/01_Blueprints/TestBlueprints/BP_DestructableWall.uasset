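; BP_DestructableWall is a test Blueprint for a wall that collapses when its OnDestruction event is called.
; The event runs its effect once, guarded by the GatesOpen flag, turning on physics simulation for the Cube's static mesh children and the Cube itself.
; It also disables collision on the Box component when it breaks apart.
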(event EventBeginPlay)

(event Collision|EventActorBeginOverlap
  (params (OtherActor :type Actor%20Object%20Reference)))

(event EventTick
  (params (DeltaSeconds :type Float%20%28single-precision%29)))

(event EventOnDestruction
  (params (PlayerCharacter :type Player%20Character%20Object%20Reference))
  (if (not (Variables|Default|GetbGatesOpen))
    (for _array_element (Components|GetChildrenComponents (Variables|Default|GetCube) true)
      (bind _asstatic_mesh_component (Utilities|Casting|CastToStaticMeshComponent _array_element))
      (Physics|SetSimulatePhysics _asstatic_mesh_component true))
    (Collision|SetCollisionEnabled (Variables|Default|GetBox) "NoCollision")
    (Variables|Default|SetbGatesOpen true)
    (Physics|SetSimulatePhysics (Variables|Default|GetCube) true)))

(fn ConstructionScript)