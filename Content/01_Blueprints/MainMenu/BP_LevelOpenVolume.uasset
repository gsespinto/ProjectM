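; Trigger volume that opens another level when a player character walks into it.
; On overlap it stores the character type, Agile or otherwise Berserker, in the Venari game instance.
; It then shows the loading screen widget, waits briefly, opens the configured LevelToLoad by object reference and sets input to game only.
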(event EventBeginPlay)

(event Collision|EventActorBeginOverlap
  (params (OtherActor :type Actor%20Object%20Reference))
  (bind _asplayer_character (Utilities|Casting|CastToPlayerCharacter OtherActor))
  (Utilities|FlowControl|Sequence
    (:then_0
      (Utilities|Casting|CastToAgileCharacter _asplayer_character
        (:then
          (Variables|/Script/ProjectM.VenariGameInstance|SetCurrentCharacter (CallFunction|GetVenariGameInstance) "AGILE"))
        (:CastFailed
          (Variables|/Script/ProjectM.VenariGameInstance|SetCurrentCharacter (CallFunction|GetVenariGameInstance) "BERSERKER"))))
    (:then_1
      (bind _returnvalue (UserInterface|CreateWidget "/Game/01_Blueprints/MainMenu/WBP_LoadingScreen.WBP_LoadingScreen_C"))
      (UserInterface|Viewport|AddtoViewport _returnvalue 0)
      (Utilities|FlowControl|Delay 1.0)
      (Game|OpenLevel(byObjectReference) (Variables|Default|GetLevelToLoad))
      (Input|SetInputModeGameOnly (Game|GetPlayerController 0)))))

(event EventTick
  (params (DeltaSeconds :type Float%20%28single-precision%29)))

(fn ConstructionScript)