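; BP_Giant is a Train Yard enemy that can vomit and spawn AI minions from its mouth.
; Vomit plays a montage on the mesh, and SpawnMinions spawns a random number of minions at the Mouth transform with their behavior tree.
; Neither function calls the other or is called within this Blueprint.
; BeginPlay, Tick and the construction script only defer to the parent class.
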(event EventBeginPlay
  (|CallParentFunction))

(event Collision|EventActorBeginOverlap
  (params (OtherActor :type Actor%20Object%20Reference)))

(event EventTick
  (params (DeltaSeconds :type Float%20%28single-precision%29))
  (|CallParentFunction DeltaSeconds))

(fn ConstructionScript
  (|CallParentFunction))

(fn SpawnMinions
  (bind _mouth (Variables|Default|GetMouth))
  (bind _returnvalue (Transformation|GetWorldTransform _mouth))
  (for _index (range 0 (Math|Random|RandomInteger (Variables|Default|GetSpawnRange)))
    (AI|SpawnAIFromClass (Variables|Default|GetMinionBP) (Variables|Default|GetMinionBT) (.location _returnvalue) (.rotation _returnvalue) false 0)))

(fn Vomit
  (Animation|Montage|MontagePlay (Components|SkeletalMesh|GetAnimInstance (Variables|Character|GetMesh)) (Variables|Default|GetVomitMontage) 1.0 "MontageLength" 0.0 true))